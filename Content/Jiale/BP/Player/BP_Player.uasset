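; Player character that moves relative to control yaw, can turn toward a target point, and casts mana-costing fireballs.
; BeginPlay creates the HUD and copies HP, mana and fire stats from GIBP.
; Casting checks cooldown and mana, playing UI warnings on failure, then spawns BP_Fireball on input completion.
; Looping timers, paused until needed, handle cooldown and mana regen, though nothing here starts regen; death only prints GameOver.
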(event EventBeginPlay
  ;[1 1 1] Add Player UI
  (bind _returnvalue (UserInterface|CreateWidget "/Game/Jiale/UI/WBP_Player.WBP_Player_C"))
  (bind _output_get (Variables|Default|SetUI _returnvalue))
  (UserInterface|Viewport|AddtoViewport _output_get 0)
  ;[1 1 1] Get game instance reference
  (bind _asgibp (Utilities|Casting|CastToGIBP (Game|GetGameInstance)))
  (bind _output_get_2 (Variables|Default|SetGameInstance _asgibp))
  (Utilities|FlowControl|Sequence
    (:then_0
      ;[1 1 1] Set HP
      (bind _output_get_3 (Variables|Default|SetMaxHP (Variables|/Game/Jiale/BP/GIBP.GIBP_C|GetPlayerMaxHP _output_get_2)))
      (Variables|Default|SetHP _output_get_3)
      ;[1 1 1] Set Mana
      (bind _output_get_4 (Variables|Default|SetMaxMana (Variables|/Game/Jiale/BP/GIBP.GIBP_C|GetPlayerMaxMana _output_get_2)))
      (Variables|Default|SetMana _output_get_4)
      ;[1 1 1] Set Fire CD
      (bind _output_get_5 (Variables|Default|SetFireMaxCD (Variables|/Game/Jiale/BP/GIBP.GIBP_C|GetFireMaxCD _output_get_2)))
      (Variables|Default|SetFireCD _output_get_5)
      ;[1 1 1] Set Fire cost mana
      (Variables|Default|SetFireManaCost (Variables|/Game/Jiale/BP/GIBP.GIBP_C|GetFireManaCost _output_get_2))
      ;[1 1 1] Set fire CD's timer
      (CallFunction|BindFireCDTimer)
      (CallFunction|PauseReloadFire))
    (:then_1
      ;[1 1 1] Set mana recovery speed
      (Variables|Default|SetManaRecoverSpeed (Variables|/Game/Jiale/BP/GIBP.GIBP_C|GetManaRecoverSpeed _output_get_2))
      (CallFunction|BindManaRecoveryTimer)
      (CallFunction|PauseRecoverMana))))

(event Collision|EventActorBeginOverlap
  (params (OtherActor :type Actor%20Object%20Reference)))

(event EventTick
  (params (DeltaSeconds :type Float%20%28single-precision%29)))

(event Input|EnhancedActionEvents|EnhancedInputActionIA_Move
  (params (ActionValue :type Vector%202D%20Structure) (ElapsedSeconds :type Float%20%28double-precision%29) (TriggeredSeconds :type Float%20%28double-precision%29) (InputAction :type Input%20Action%20Object%20Reference :default "/Game/Jiale/Input/IA_Move.IA_Move"))
  (bind _returnvalue (Pawn|GetControlRotation :!class /Script/Engine.Pawn))
  (bind _returnvalue_2 (Math|Rotator|MakeRotator 0.0 0.0 (.yaw _returnvalue)))
  ;[1 1 1] Move forward and right
  (:Triggered
    (Utilities|FlowControl|Sequence
      (:then_0
        (Pawn|Input|AddMovementInput (Math|Vector|GetForwardVector _returnvalue_2) (.y ActionValue) false))
      (:then_1
        (Pawn|Input|AddMovementInput (Math|Vector|GetRightVector _returnvalue_2) (.x ActionValue) false)))))

(event EventLookat
  (params (Target :type Vector :default "0, 0, 0"))
  (bind _returnvalue (Transformation|GetActorLocation))
  ;[1 1 1] Look at the cursor location
  (Transformation|SetActorRotation (Math|Rotator|FindLookatRotation (Math|Vector|MakeVector (.x _returnvalue) (.y _returnvalue) 0.0) (Math|Vector|MakeVector (.x Target) (.y Target) 0.0))))

(event Custom|StartReloadFire
  ;[1 1 1] Fireball reload events
  ;;[1 1 1] Start timer
  (Utilities|Time|UnpauseTimerbyHandle (stale Custom|BindFireCDTimer _returnvalue)))

(event Custom|ReloadingFire
  ;[1 1 1] Fireball reload events
  ;;[1 1 1] Reloading
  (if (>= (Variables|Default|GetFireCD) (Variables|Default|GetFireMaxCD))
    (Variables|Default|SetFireReloaded true)
    (CallFunction|PauseReloadFire)
    (else
      (Variables|Default|SetFireCD (Math|Float|Clamp(Float) (+ (Variables|Default|GetFireCD) 0.1) 0.0 (Variables|Default|GetFireMaxCD))))))

(event Custom|BindFireCDTimer
  ;[1 1 1] Fireball reload events
  ;;[1 1 1] Binding Timer
  (bind _returnvalue (Utilities|Time|SetTimerbyEvent (delegate Custom|ReloadingFire) 0.1 true)))

(event Custom|PauseReloadFire
  ;[1 1 1] Fireball reload events
  ;;[1 1 1] Pause timer
  (Utilities|Time|PauseTimerbyHandle (stale Custom|BindFireCDTimer _returnvalue)))

(event Custom|BindManaRecoveryTimer
  ;[1 1 1] Recover mana
  ;;[1 1 1] Binding
  (bind _returnvalue (Utilities|Time|SetTimerbyEvent (delegate Custom|RecoveringMana) 1.0 true)))

(event Custom|RecoveringMana
  ;[1 1 1] Recover mana
  ;;[1 1 1] Recovering
  (if (>= (Variables|Default|GetMana) (Variables|Default|GetMaxMana))
    (CallFunction|PauseRecoverMana)
    (else
      (Variables|Default|SetMana (Math|Integer|Clamp(Integer) (+ (Variables|Default|GetMana) (Variables|Default|GetManaRecoverSpeed)) 0 (Variables|Default|GetMaxMana))))))

(event Custom|StartRecoverMana
  ;[1 1 1] Recover mana
  ;;[1 1 1] Start
  (Utilities|Time|UnpauseTimerbyHandle (stale Custom|BindManaRecoveryTimer _returnvalue)))

(event Custom|PauseRecoverMana
  ;[1 1 1] Recover mana
  ;;[1 1 1] Pause
  (Utilities|Time|PauseTimerbyHandle (stale Custom|BindManaRecoveryTimer _returnvalue)))

(event Input|EnhancedActionEvents|EnhancedInputActionIA_SpellMagic
  (params (ActionValue :type Boolean) (ElapsedSeconds :type Float%20%28double-precision%29) (TriggeredSeconds :type Float%20%28double-precision%29) (InputAction :type Input%20Action%20Object%20Reference :default "/Game/Jiale/Input/IA_SpellMagic.IA_SpellMagic"))
  (:Started
    (bind _iscanfire (CallFunction|CheckManatoFire))
    (Variables|Default|SetIsFireAiming _iscanfire))
  (:Ongoing
    (if (Variables|Default|GetIsFireAiming)
      _))
  (:Completed
    (if (Variables|Default|GetIsFireAiming)
      (Variables|Default|SetIsSpellingFire true)
      (Variables|Default|SetFireReloaded false)
      (CallFunction|UpdateMana (Variables|Default|GetFireManaCost) true)
      (Variables|Default|SetFireCD 0.0)
      (CallFunction|StartReloadFire)
      (Utilities|FlowControl|Delay 0.5)
      (Game|SpawnActorfromClass "/Game/Jiale/BP/Player/BP_Fireball.BP_Fireball_C" (Math|Transform|MakeTransform (.location (Transformation|GetWorldTransform (Variables|Default|GetFIreballShootLocation))) "0, 0, 0" "1.000000,1.000000,1.000000") "Undefined" "MultiplyWithRoot" 0 0)
      (Utilities|FlowControl|Delay 0.5)
      (Variables|Default|SetIsSpellingFire false))))

(event EventGetDamage
  (params (Damage :type Integer))
  ;[1 1 1] Calculate HP when player get damage
  (CallFunction|UpdateHP Damage true)
  (bind _isdying (CallFunction|CheckLife))
  (if _isdying
    (Utilities|FlowControl|Delay 1.0)
    (Development|PrintString "GameOver")))

(fn ConstructionScript)

(fn UpdateHP
  (params (DeltaHP :type Integer) (IsDamage :type Boolean))
  (if IsDamage
    ;[1 1 1] Get damage
    (Variables|Default|SetHP (Math|Integer|Clamp(Integer) (- (Variables|Default|GetHP) DeltaHP) 0 (Variables|Default|GetMaxHP)))
    (else
      ;[1 1 1] Get Recovery
      (Variables|Default|SetHP (Math|Integer|Clamp(Integer) (+ (Variables|Default|GetHP) DeltaHP) 0 (Variables|Default|GetMaxHP))))))

(fn CheckLife
  (if (<= (Variables|Default|GetHP) 0)
    (bind _output_get (Variables|Default|SetIsDying true))
    (return _output_get)
    (else
      (bind _output_get_2 (Variables|Default|SetIsDying false))
      (return _output_get_2))))

(fn UpdateMana
  (params (DeltaMana :type Integer) (IsCost :type Boolean))
  (if IsCost
    ;[1 1 1] Cost Mana
    (Variables|Default|SetMana (Math|Integer|Clamp(Integer) (- (Variables|Default|GetMana) DeltaMana) 0 (Variables|Default|GetMaxMana)))
    (else
      ;[1 1 1] Recovery Mana
      (Variables|Default|SetMana (Math|Integer|Clamp(Integer) (+ (Variables|Default|GetMana) DeltaMana) 0 (Variables|Default|GetMaxMana))))))

(fn CheckManatoFire
  (bind _ui (Variables|Default|GetUI))
  (bind _ui_2 (Variables|Default|GetUI))
  (if (Variables|Default|GetFireReloaded)
    (if (>= (Variables|Default|GetMana) (Variables|Default|GetFireManaCost))
      (return true)
      (else
        (UserInterface|Animation|PlayAnimation _ui (Variables|/Game/Jiale/UI/WBP_Player.WBP_Player_C|GetOutOfMana _ui) 0.0 1 "Forward" 1.0 false)))
    (else
      (UserInterface|Animation|PlayAnimation _ui_2 (Variables|/Game/Jiale/UI/WBP_Player.WBP_Player_C|GetAttackOnCD _ui_2) 0.0 1 "Forward" 1.0 false)))
  (return false))