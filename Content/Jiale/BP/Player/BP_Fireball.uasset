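; BP_Fireball is a player projectile that arcs to the mouse location and explodes on impact.
; On BeginPlay it gets the target from BP_PlayerController, solves the arc with SuggestProjectileVelocityCustomArc and passes the result to ProjectileMovement as local-space velocity.
; A collision hit with a valid actor spawns BP_Explosion and destroys the fireball.
; A successful launch also starts a timed self-destruct as a lifetime cap.
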(event OnComponentHit(Collision)
  (params (HitComponent :type Primitive%20Component%20Object%20Reference) (OtherActor :type Actor%20Object%20Reference) (OtherComp :type Primitive%20Component%20Object%20Reference) (NormalImpulse :type Vector :default "0, 0, 0") (Hit :type Hit%20Result%20Structure%20%28by%20ref%29))
  ;[1 1 1] If fire ball hits the ground
  (Utilities|IsValid OtherActor
    (:Is%20Valid
      ;[1 1 1] Spawn explosion
      (Game|SpawnActorfromClass "/Game/Jiale/BP/Player/BP_Explosion.BP_Explosion_C" (Math|Transform|MakeTransform (Transformation|GetWorldLocation (Variables|Default|GetSphere)) "0, 0, 0" "1.000000,1.000000,1.000000") "Undefined" "MultiplyWithRoot" 0 0)
      ;[1 1 1] Destroy Fireball
      (Actor|DestroyActor))))

(event EventBeginPlay
  ;[1 1 1] Get mouse location
  (bind _asbp_player_controller (Utilities|Casting|CastToBP_PlayerController (Game|GetPlayerController 0)))
  (bind _target (Default|GetMouseLocation _asbp_player_controller))
  ;[1 1 1] Set fireball's route
  (bind (_outlaunchvelocity _returnvalue) (Game|SuggestProjectileVelocityCustomArc (Transformation|GetWorldLocation (Variables|Default|GetSphere)) _target 0.0 0.5))
  (if _returnvalue
    (Game|Components|ProjectileMovement|SetVelocityinLocalSpace (Variables|Default|GetProjectileMovement) _outlaunchvelocity)
    ;[1 1 1] Max life time is 10 seconds
    (Utilities|FlowControl|Delay 1e+01)
    (Actor|DestroyActor)))

(fn ConstructionScript)