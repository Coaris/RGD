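; GIBP, apparently the Game Instance, holds player and home base stats and provides the gold-bought upgrade and repair events.
; Each event deducts its cost from PlayerGold, then steps one stat and clamps it: fire damage, mana cost, cooldown, max HP, max mana, mana recovery or base health.
; No event checks affordability or whether the stat is already at its limit, so gold is spent regardless.
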(event Custom|Up_FireDamage
  (Variables|Default|SetPlayerGold (- (Variables|Default|GetPlayerGold) (Variables|Default|GetUp_FireDamage_Cost)))
  (bind _result (Math|Integer|IncrementInt (Variables|Default|GetFireDamage))
    (:%20%20
      (Variables|Default|SetFireDamage (Math|Integer|Clamp(Integer) _result 1 20)))))

(event Custom|Up_FireManaCost
  (Variables|Default|SetPlayerGold (- (Variables|Default|GetPlayerGold) (Variables|Default|GetUp_FireManaCost_Cost)))
  (bind _result (Math|Integer|DecrementInt (Variables|Default|GetFireManaCost))
    (:%20%20
      (Variables|Default|SetFireManaCost (Math|Integer|Clamp(Integer) _result 2 10)))))

(event Custom|Up_FireMaxCD
  (Variables|Default|SetPlayerGold (- (Variables|Default|GetPlayerGold) (Variables|Default|GetUp_FireMaxCD_Cost)))
  (Variables|Default|SetFireMaxCD (Math|Float|Clamp(Float) (- (Variables|Default|GetFireMaxCD) 0.1) 1.0 1e+01)))

(event Custom|Up_MaxHP
  (Variables|Default|SetPlayerGold (- (Variables|Default|GetPlayerGold) (Variables|Default|GetUP_MaxHP_Cost)))
  (bind _result (Math|Integer|IncrementInt (Variables|Default|GetPlayerMaxHP))
    (:%20%20
      (Variables|Default|SetPlayerMaxHP (Math|Integer|Clamp(Integer) _result 1 20)))))

(event Custom|Up_MaxMana
  (Variables|Default|SetPlayerGold (- (Variables|Default|GetPlayerGold) (Variables|Default|GetUp_MaxMana_Cost)))
  (bind _result (Math|Integer|IncrementInt (Variables|Default|GetPlayerMaxMana))
    (:%20%20
      (Variables|Default|SetPlayerMaxMana (Math|Integer|Clamp(Integer) _result 5 50)))))

(event Custom|Up_ManaRecoverSpeed
  (Variables|Default|SetPlayerGold (- (Variables|Default|GetPlayerGold) (Variables|Default|GetUP_ManaRecoverSpeed_Cost)))
  (bind _result (Math|Integer|IncrementInt (Variables|Default|GetManaRecoverSpeed))
    (:%20%20
      (Variables|Default|SetManaRecoverSpeed (Math|Integer|Clamp(Integer) _result 1 5)))))

(event Custom|FixBaseHealth
  (Variables|Default|SetPlayerGold (- (Variables|Default|GetPlayerGold) (Variables|Default|GetFixBaseHealth_Cost)))
  (Variables|Default|SetHomeHP (Math|Integer|Clamp(Integer) (+ (Variables|Default|GetHomeHP) 1) 0 (Variables|Default|GetHomeMaxHP))))