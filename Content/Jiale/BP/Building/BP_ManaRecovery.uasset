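; BP_ManaRecovery is a building that restores the player's mana while the player is inside its sphere.
; On BeginPlay it caches the first player pawn as a BP_Player reference.
; Sphere overlap begin and end, filtered to BP_Player actors, call StartRecoverMana and PauseRecoverMana on that cached player, which handles the recovery itself.
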(event OnComponentBeginOverlap(Sphere)
  (params (OverlappedComponent :type Primitive%20Component%20Object%20Reference) (OtherActor :type Actor%20Object%20Reference) (OtherComp :type Primitive%20Component%20Object%20Reference) (OtherBodyIndex :type Integer) (bFromSweep :type Boolean) (SweepResult :type Hit%20Result%20Structure%20%28by%20ref%29))
  ;[1 1 1] Recover mana
  (Utilities|Casting|CastToBP_Player OtherActor)
  (Default|StartRecoverMana (Variables|Default|GetPlayer)))

(event OnComponentEndOverlap(Sphere)
  (params (OverlappedComponent :type Primitive%20Component%20Object%20Reference) (OtherActor :type Actor%20Object%20Reference) (OtherComp :type Primitive%20Component%20Object%20Reference) (OtherBodyIndex :type Integer))
  ;[1 1 1] Pause recover mana
  (Utilities|Casting|CastToBP_Player OtherActor)
  (Default|PauseRecoverMana (Variables|Default|GetPlayer)))

(event EventBeginPlay
  ;[1 1 1] Get player reference
  (bind _asbp_player (Utilities|Casting|CastToBP_Player (Game|Player|GetPlayerPawn 0)))
  (Variables|Default|SetPlayer _asbp_player))

(fn ConstructionScript)