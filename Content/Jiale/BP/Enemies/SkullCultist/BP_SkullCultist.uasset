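; BP_SkullCultist is a healer enemy that walks toward BP_Home, with stats loaded from the game instance.
; Looping timers drive AI movement and an IsAttacking pulse, while HealSkill spawns a BP_HealRange.
; Overlaps with BP_Explosion damage it and BP_HealRange heals it, updating a health bar widget.
; Death awards gold and score, then teleports it to its start to respawn, or notifies BP_LevelCheck and destroys it once respawns run out.
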(event OnComponentBeginOverlap(CapsuleComponent)
  (params (OverlappedComponent :type Primitive%20Component%20Object%20Reference) (OtherActor :type Actor%20Object%20Reference) (OtherComp :type Primitive%20Component%20Object%20Reference) (OtherBodyIndex :type Integer) (bFromSweep :type Boolean) (SweepResult :type Hit%20Result%20Structure%20%28by%20ref%29))
  (bind _gameinstance (Variables|Default|GetGameInstance))
  (bind _respawned (Variables|Default|GetRespawned))
  (bind _gameinstance_2 (Variables|Default|GetGameInstance))
  ;[1 1 1] Get damage from player
  (Utilities|Casting|CastToBP_Explosion OtherActor
    (:then
      (CallFunction|UpdateHP (Variables|/Game/Jiale/BP/GIBP.GIBP_C|GetFireDamage (Variables|Default|GetGameInstance)) true)
      (bind _isdying (CallFunction|CheckLife))
      (Utilities|FlowControl|Delay 0.2)
      (if _isdying
        ;;[1 1 1] player get coin
        (Variables|/Game/Jiale/BP/GIBP.GIBP_C|SetPlayerGold _gameinstance (+ (Variables|/Game/Jiale/BP/GIBP.GIBP_C|GetPlayerGold _gameinstance) (Variables|/Game/Jiale/BP/GIBP.GIBP_C|GetSkullGold _gameinstance)))
        ;;[1 1 1] Player get score
        (Variables|/Game/Jiale/BP/GIBP.GIBP_C|SetPlayerScore _gameinstance_2 (+ (Variables|/Game/Jiale/BP/GIBP.GIBP_C|GetPlayerScore _gameinstance_2) (Variables|/Game/Jiale/BP/GIBP.GIBP_C|GetSkullScore _gameinstance_2)))
        (Development|SetHiddeninGame (Variables|Default|GetWidget) true false)
        (Utilities|FlowControl|Delay 1.0)
        (if (< _respawned (Variables|Default|GetRespawnTimes))
          (Math|Integer|IncrementInt _respawned
            (:%20%20
              (Transformation|SetActorLocation (Variables|Default|GetStartLocation) false false)
              (Variables|Default|SetIsDying false)
              (Development|SetHiddeninGame (Variables|Default|GetWidget) false false)
              (CallFunction|UpdateHP (Variables|Default|GetMaxHP) false)))
          (else
            (bind _returnvalue (Actor|GetActorOfClass "/Game/Jiale/BP/BP_LevelCheck.BP_LevelCheck_C"))
            (Class|BPILevelCheck|SkullDead(Message) _returnvalue)
            (Actor|DestroyActor)))
        (Default|CalcRemaining (Variables|Default|GetGameInstance))))
    (:CastFailed
      (Utilities|Casting|CastToBP_HealRange OtherActor)
      (CallFunction|UpdateHP (Variables|/Game/Jiale/BP/GIBP.GIBP_C|GetSkullAttack (Variables|Default|GetGameInstance)) false))))

(event Custom|MoveToHome
  ;[1 1 1] Go to home
  (AI|AIMoveTo self "0, 0, 0" (Variables|Default|GetHome) 6.5e+02 false))

(event Custom|Heal
  ;[1 1 1] Heal Skell
  (if (not (Variables|Default|GetIsAttacking))
    (Variables|Default|SetIsAttacking true)
    (Utilities|FlowControl|Delay 1.0)
    (Variables|Default|SetIsAttacking false)))

(event Custom|HealSkill
  ;[1 1 1] Heal
  (Game|SpawnActorfromClass "/Game/Jiale/BP/Enemies/SkullCultist/BP_HealRange.BP_HealRange_C" (Transformation|GetWorldTransform (Variables|Collision|GetCapsuleComponent)) "Undefined" "MultiplyWithRoot" 0 0))

(event EventBeginPlay
  (Utilities|FlowControl|Sequence
    (:then_0
      ;[1 1 1] Get game instance reference
      (bind _asgibp (Utilities|Casting|CastToGIBP (Game|GetGameInstance)))
      (bind _output_get (Variables|Default|SetGameInstance _asgibp))
      (bind _output_get_2 (Variables|Default|SetMaxHP (Variables|/Game/Jiale/BP/GIBP.GIBP_C|GetSkullMaxHP _output_get)))
      (Variables|Default|SetHP _output_get_2)
      ;[1 1 1] Get home reference
      (bind _returnvalue (Actor|GetActorOfClass "/Game/Jiale/BP/Building/BP_Home.BP_Home_C"))
      (Variables|Default|SetHome _returnvalue)
      ;[1 1 1] Set start location
      (Variables|Default|SetStartLocation (Transformation|GetWorldLocation (Variables|Collision|GetCapsuleComponent))))
    (:then_1
      ;[1 1 1] Get attack
      (Variables|Default|SetAttack (Variables|/Game/Jiale/BP/GIBP.GIBP_C|GetSkullAttack (Variables|Default|GetGameInstance)))
      ;[1 1 1] Get attack speed
      (Variables|Default|SetAttackSpeed (Variables|/Game/Jiale/BP/GIBP.GIBP_C|GetSkullAttackSpeed (Variables|Default|GetGameInstance))))
    (:then_2
      ;[1 1 1] Go to home
      (Utilities|Time|SetTimerbyEvent (delegate Custom|MoveToHome) 2.0 true))
    (:then_3
      ;[1 1 1] Heal Skell
      (Utilities|Time|SetTimerbyEvent (delegate Custom|Heal) (Variables|Default|GetAttackSpeed) true))
    (:then_4
      ;[1 1 1] Get respawn times
      (Utilities|FlowControl|Delay 1.0)
      (Variables|Default|SetRespawnTimes (Variables|/Game/Jiale/BP/GIBP.GIBP_C|GetSkullRespawnTimes (Variables|Default|GetGameInstance)))
      (Variables|Default|SetRespawned 1))))

(fn ConstructionScript)

(fn UpdateHP
  (params (DeltaHP :type Integer) (IsDamage :type Boolean))
  (if IsDamage
    ;[1 1 1] Get damage
    (Variables|Default|SetHP (Math|Integer|Clamp(Integer) (- (Variables|Default|GetHP) DeltaHP) 0 (Variables|Default|GetMaxHP)))
    (else
      ;[1 1 1] Get Recovery
      (Variables|Default|SetHP (Math|Integer|Clamp(Integer) (+ (Variables|Default|GetHP) DeltaHP) 0 (Variables|Default|GetMaxHP)))))
  ;[1 1 1] Change HealthBar
  (bind _aswbp_health_bar (Utilities|Casting|CastToWBP_HealthBar (UserInterface|GetWidget (Variables|Default|GetWidget))))
  (Progress|SetPercent (Variables|/Game/Jiale/UI/WBP_HealthBar.WBP_HealthBar_C|GetHealthBar _aswbp_health_bar) (/ (Variables|Default|GetHP) (Variables|Default|GetMaxHP))))

(fn CheckLife
  (if (<= (Variables|Default|GetHP) 0)
    (bind _output_get (Variables|Default|SetIsDying true))
    (return _output_get)
    (else
      (bind _output_get_2 (Variables|Default|SetIsDying false))
      (return _output_get_2))))