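; BP_EvilSkeleton is an enemy skeleton that takes damage from explosions and rewards the player when it dies.
; On BeginPlay it caches the game instance (GIBP) and initializes its health from it.
; Capsule overlaps with BP_Explosion apply the game instance's fire damage through a clamped UpdateHP, then CheckLife flags death.
; On death, short delays precede adding gold and score to the game instance and destroying the actor.
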(event OnComponentBeginOverlap(CapsuleComponent)
  (params (OverlappedComponent :type Primitive%20Component%20Object%20Reference) (OtherActor :type Actor%20Object%20Reference) (OtherComp :type Primitive%20Component%20Object%20Reference) (OtherBodyIndex :type Integer) (bFromSweep :type Boolean) (SweepResult :type Hit%20Result%20Structure%20%28by%20ref%29))
  (bind _gameinstance (Variables|Default|GetGameInstance))
  (bind _gameinstance_2 (Variables|Default|GetGameInstance))
  ;[1 1 1] Get damage from player
  (Utilities|Casting|CastToBP_Explosion OtherActor)
  (CallFunction|UpdateHP (Variables|/Game/Jiale/BP/GIBP.GIBP_C|GetFireDamage (Variables|Default|GetGameInstance)) true)
  (bind _isdying (CallFunction|CheckLife))
  (Utilities|FlowControl|Delay 0.2)
  (if _isdying
    ;;[1 1 1] player get coin
    (Variables|/Game/Jiale/BP/GIBP.GIBP_C|SetPlayerGold _gameinstance (+ (Variables|/Game/Jiale/BP/GIBP.GIBP_C|GetPlayerGold _gameinstance) (Variables|/Game/Jiale/BP/GIBP.GIBP_C|GetEvilGold _gameinstance)))
    ;;[1 1 1] Player get score
    (Variables|/Game/Jiale/BP/GIBP.GIBP_C|SetPlayerScore _gameinstance_2 (+ (Variables|/Game/Jiale/BP/GIBP.GIBP_C|GetPlayerScore _gameinstance_2) (Variables|/Game/Jiale/BP/GIBP.GIBP_C|GetEvilScore _gameinstance_2)))
    (Utilities|FlowControl|Delay 1.0)
    (Actor|DestroyActor)))

(event EventBeginPlay
  ;[1 1 1] Get game instance reference
  (bind _asgibp (Utilities|Casting|CastToGIBP (Game|GetGameInstance)))
  (bind _output_get (Variables|Default|SetGameInstance _asgibp))
  (bind _output_get_2 (Variables|Default|SetMaxHP (Variables|/Game/Jiale/BP/GIBP.GIBP_C|GetEvilMaxHP _output_get)))
  (Variables|Default|SetHP _output_get_2))

(fn ConstructionScript)

(fn UpdateHP
  (params (DeltaHP :type Integer) (IsDamage :type Boolean))
  (if IsDamage
    ;[1 1 1] Get damage
    (Variables|Default|SetHP (Math|Integer|Clamp(Integer) (- (Variables|Default|GetHP) DeltaHP) 0 (Variables|Default|GetMaxHP)))
    (else
      ;[1 1 1] Get Recovery
      (Variables|Default|SetHP (Math|Integer|Clamp(Integer) (+ (Variables|Default|GetHP) DeltaHP) 0 (Variables|Default|GetMaxHP))))))

(fn CheckLife
  (if (<= (Variables|Default|GetHP) 0)
    (bind _output_get (Variables|Default|SetIsDying true))
    (return _output_get)
    (else
      (bind _output_get_2 (Variables|Default|SetIsDying false))
      (return _output_get_2))))