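; BP_waterball is an enemy attack actor in the EvilSkeleton folder that damages the player or the home on overlap.
; Its Box overlap sends the game instance's EvilAttack damage to BP_Player and then destroys the ball.
; A BP_Home hit subtracts that damage from the shared, clamped HomeHP and triggers a home life check, without destroying the ball.
; The actor also destroys itself after a fixed delay from BeginPlay.
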(event OnComponentBeginOverlap(Box)
  (params (OverlappedComponent :type Primitive%20Component%20Object%20Reference) (OtherActor :type Actor%20Object%20Reference) (OtherComp :type Primitive%20Component%20Object%20Reference) (OtherBodyIndex :type Integer) (bFromSweep :type Boolean) (SweepResult :type Hit%20Result%20Structure%20%28by%20ref%29))
  (bind _gameinstance (Variables|Default|GetGameInstance))
  (bind _gameinstance_2 (Variables|Default|GetGameInstance))
  (bind _evilattack (Variables|/Game/Jiale/BP/GIBP.GIBP_C|GetEvilAttack _gameinstance))
  ;[1 1 1] Damage on Player and home
  (bind _asbp_player (Utilities|Casting|CastToBP_Player OtherActor)
    (:then
      (Class|BPIPlayer|GetDamage(Message) _asbp_player _evilattack)
      (Actor|DestroyActor))
    (:CastFailed
      (bind _asbp_home (Utilities|Casting|CastToBP_Home OtherActor))
      (Variables|/Game/Jiale/BP/GIBP.GIBP_C|SetHomeHP _gameinstance_2 (Math|Integer|Clamp(Integer) (- (Variables|/Game/Jiale/BP/GIBP.GIBP_C|GetHomeHP _gameinstance_2) _evilattack) 0 100))
      (Class|BPIHome|CheckHomeLife(Message) _asbp_home))))

(event EventBeginPlay
  ;[1 1 1] Get game instance reference and destroy in 10 seconds
  (bind _asgibp (Utilities|Casting|CastToGIBP (Game|GetGameInstance)))
  (Variables|Default|SetGameInstance _asgibp)
  (Utilities|FlowControl|Delay 1e+01)
  (Actor|DestroyActor))

(fn ConstructionScript)