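; Player controller Blueprint that shows the mouse cursor, feeds cursor aim to the player pawn and handles the pause menu.
; Each Tick, a complex Visibility trace under the cursor sends its hit location to the pawn via LookAtMessage.
; IA_PauseGame toggles WBP_PauseMenu and the input mode, though both branches call SetGamePaused(true), so the resume branch leaves the game paused.
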(event Input|EnhancedActionEvents|EnhancedInputActionIA_PauseGame
  (params (ActionValue :type Boolean) (ElapsedSeconds :type Float%20%28double-precision%29) (TriggeredSeconds :type Float%20%28double-precision%29) (InputAction :type Input%20Action%20Object%20Reference :default "/Game/Jiale/Input/IA_PauseGame.IA_PauseGame"))
  (bind _returnvalue (Game|GetPlayerController 0))
  (:Started
    (if (Variables|Default|GetIsPaused)
      ;[1 1 1] Resume
      (Variables|Default|SetIsPaused false)
      (Widget|RemovefromParent (Variables|Default|GetPauseMenu))
      (Game|SetGamePaused true)
      (Input|SetInputModeGameOnly _returnvalue false)
      (else
        ;[1 1 1] Pause
        (Variables|Default|SetIsPaused true)
        (bind _returnvalue_2 (UserInterface|CreateWidget "/Game/Jiale/UI/WBP_PauseMenu.WBP_PauseMenu_C" _returnvalue))
        (bind _output_get (Variables|Default|SetPauseMenu _returnvalue_2))
        (UserInterface|Viewport|AddtoViewport _output_get 0)
        (Input|SetInputModeGameandUI _returnvalue (Variables|Default|GetPauseMenu) "DoNotLock" true false)
        (Game|SetGamePaused true)))))

(event EventBeginPlay
  (Variables|Default|SetbShowMouseCursor true))

(event EventTick
  (params (DeltaSeconds :type Float%20%28single-precision%29))
  ;[1 1 1] Get Cursor location
  (Class|BPIPlayer|Lookat(Message) (Game|Player|GetPlayerPawn 0) (.location (.HitResult (Game|Player|GetHitResultUnderCursorbyChannel "TraceTypeQuery1" true)))))

(fn ConstructionScript)

(fn GetMouseLocation
  (return (.location (.HitResult (Game|Player|GetHitResultUnderCursorbyChannel "TraceTypeQuery1" true)))))