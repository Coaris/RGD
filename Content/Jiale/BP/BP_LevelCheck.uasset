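; BP_LevelCheck is a level actor that tracks whether all ghost, evil skeleton and skull cultist enemies are dead.
; BeginPlay counts each enemy class in the level, and the matching death events decrement those counts and run CheckEnd.
; CheckEnd only prints "NextLevel" when all three reach zero.
; A separate GoToNextLevel event, not called here, increments WaveNumber in the GIBP game instance and opens the next level.
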(event Custom|GoToNextLevel
  (bind _asgibp (Utilities|Casting|CastToGIBP (Game|GetGameInstance)))
  (Math|Integer|IncrementInt (Variables|/Game/Jiale/BP/GIBP.GIBP_C|GetWaveNumber _asgibp)
    (:%20%20
      (Game|OpenLevel(byName) (Variables|Default|GetNextLevel)))))

(event EventBeginPlay
  (Utilities|FlowControl|Sequence
    (:then_0
      (bind _outactors (Actor|GetAllActorsOfClass "/Game/Jiale/BP/Enemies/Ghost/BP_Enemy_Ghost.BP_Enemy_Ghost_C"))
      (Variables|Default|SetGhostAmount (Utilities|Array|Length _outactors)))
    (:then_1
      (bind _outactors_2 (Actor|GetAllActorsOfClass "/Game/Jiale/BP/Enemies/EvilSkeleton/BP_EvilSkeleton.BP_EvilSkeleton_C"))
      (Variables|Default|SetEvilAmount (Utilities|Array|Length _outactors_2)))
    (:then_2
      (bind _outactors_3 (Actor|GetAllActorsOfClass "/Game/Jiale/BP/Enemies/SkullCultist/BP_SkullCultist.BP_SkullCultist_C"))
      (Variables|Default|SetSkullAmount (Utilities|Array|Length _outactors_3)))))

(event EventEvilDead
  (Math|Integer|DecrementInt (Variables|Default|GetEvilAmount)
    (:%20%20
      (CallFunction|CheckEnd))))

(event EventGhostDead
  (Math|Integer|DecrementInt (Variables|Default|GetGhostAmount)
    (:%20%20
      (CallFunction|CheckEnd))))

(event EventSkullDead
  (Math|Integer|DecrementInt (Variables|Default|GetSkullAmount)
    (:%20%20
      (CallFunction|CheckEnd))))

(fn ConstructionScript)

(fn CheckEnd
  (if (== (Variables|Default|GetGhostAmount) 0)
    (if (== (Variables|Default|GetEvilAmount) 0)
      (if (== (Variables|Default|GetSkullAmount) 0)
        (Development|PrintString "NextLevel")))))